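; BP_JewelKey is a colored jewel key pickup that the third-person player character collects by touching it.
; The construction script sets the sphere's material from the KeyValue enum, so each placed instance shows its blue, green, red or yellow color.
; When the character overlaps the box, the key value is added to the set in its JKeysComponent and the pickup destroys itself.
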(event OnComponentBeginOverlap(Box)
  (params (OverlappedComponent :type Primitive%20Component%20Object%20Reference) (OtherActor :type Actor%20Object%20Reference) (OtherComp :type Primitive%20Component%20Object%20Reference) (OtherBodyIndex :type Integer) (bFromSweep :type Boolean) (SweepResult :type Hit%20Result%20Structure%20%28by%20ref%29))
  (bind _asbp_third_person_character (Utilities|Casting|CastToBP_ThirdPersonCharacter OtherActor))
  (Default|AddKeytoSet (Variables|/Game/ThirdPerson/Blueprints/BP_ThirdPersonCharacter.BP_ThirdPersonCharacter_C|GetJKeysComponent _asbp_third_person_character) (Variables|Default|GetKeyValue))
  (Actor|DestroyActor))

(event EventBeginPlay)

(event Collision|EventActorBeginOverlap
  (params (OtherActor :type Actor%20Object%20Reference)))

(event EventTick
  (params (DeltaSeconds :type Float%20%28single-precision%29)))

(fn ConstructionScript
  (bind _sphere (Variables|Default|GetSphere))
  (switch Utilities|FlowControl|Switch|SwitchonEnum_JewelKeyType (Variables|Default|GetKeyValue)
    (:NewEnumerator0
      (Rendering|Material|SetMaterial _sphere 0 "/Game/LevelPrototyping/Materials/MI_Solid_Blue.MI_Solid_Blue"))
    (:NewEnumerator1
      (Rendering|Material|SetMaterial _sphere 0 "/Game/Material/M_SampleColor_InstGreen.M_SampleColor_InstGreen"))
    (:NewEnumerator2
      (Rendering|Material|SetMaterial _sphere 0 "/Game/Material/M_SampleColor_InstRed.M_SampleColor_InstRed"))
    (:NewEnumerator3
      (Rendering|Material|SetMaterial _sphere 0 "/Game/Material/M_SampleColor_InstYellow.M_SampleColor_InstYellow"))))