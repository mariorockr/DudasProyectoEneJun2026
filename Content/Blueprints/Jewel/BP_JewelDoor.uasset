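; A jewel-locked door that opens for a player character carrying the jewel of its assigned type.
; The construction script colors the Cube mesh by JewelType: blue, green, red or yellow.
; When a BP_ThirdPersonCharacter overlaps the Box, the door checks that character's JewelComponent set for the matching type.
; On a match, a timeline moves the Cube along Z by cumulative offsets, with no closing logic.
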(event OnComponentBeginOverlap(Box)
  (params (OverlappedComponent :type Primitive%20Component%20Object%20Reference) (OtherActor :type Actor%20Object%20Reference) (OtherComp :type Primitive%20Component%20Object%20Reference) (OtherBodyIndex :type Integer) (bFromSweep :type Boolean) (SweepResult :type Hit%20Result%20Structure%20%28by%20ref%29))
  (bind _asbp_third_person_character (Utilities|Casting|CastToBP_ThirdPersonCharacter OtherActor))
  (if (Utilities|Set|Contains (Variables|/Game/Blueprints/Jewel/JewelComponent.JewelComponent_C|GetJewelSetContainer (Variables|/Game/ThirdPerson/Blueprints/BP_ThirdPersonCharacter.BP_ThirdPersonCharacter_C|GetJewelComponent _asbp_third_person_character)) (Variables|Default|GetJewelType))
    (CallFunction|OpenDoor)))

(event Custom|OpenDoor
  (bind _time (Timeline|Timeline Play)
    (:Update
      (Transformation|AddWorldOffset (Variables|Default|GetCube) (Math|Vector|MakeVector 0.0 0.0 _time) false false))))

(event EventBeginPlay)

(event Collision|EventActorBeginOverlap
  (params (OtherActor :type Actor%20Object%20Reference)))

(event EventTick
  (params (DeltaSeconds :type Float%20%28single-precision%29)))

(fn ConstructionScript
  (bind _cube (Variables|Default|GetCube))
  (switch Utilities|FlowControl|Switch|SwitchonJewelType (Variables|Default|GetJewelType)
    (:NewEnumerator0
      (Rendering|Material|SetMaterial _cube 0 "/Game/LevelPrototyping/Materials/MI_Solid_Blue.MI_Solid_Blue"))
    (:NewEnumerator1
      (Rendering|Material|SetMaterial _cube 0 "/Game/Material/M_SampleColor_InstGreen.M_SampleColor_InstGreen"))
    (:NewEnumerator2
      (Rendering|Material|SetMaterial _cube 0 "/Game/Material/M_SampleColor_InstRed.M_SampleColor_InstRed"))
    (:NewEnumerator3
      (Rendering|Material|SetMaterial _cube 0 "/Game/Material/M_SampleColor_InstYellow.M_SampleColor_InstYellow"))))