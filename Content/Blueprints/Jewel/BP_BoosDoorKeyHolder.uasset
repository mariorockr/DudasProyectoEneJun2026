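; A key holder actor that registers one colored key with a linked boss door.
; When the third-person character overlaps its box, it adds its key type to the door's activated keys and has the door update, only once.
; The construction script colors the cube blue, green, red or yellow to match the selected key type.
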(event OnComponentBeginOverlap(Box)
  (params (OverlappedComponent :type Primitive%20Component%20Object%20Reference) (OtherActor :type Actor%20Object%20Reference) (OtherComp :type Primitive%20Component%20Object%20Reference) (OtherBodyIndex :type Integer) (bFromSweep :type Boolean) (SweepResult :type Hit%20Result%20Structure%20%28by%20ref%29))
  (Utilities|Casting|CastToBP_ThirdPersonCharacter OtherActor)
  (if (not (Variables|Default|GetDidActivateKey))
    (Utilities|Set|Add (Variables|/Game/Blueprints/Jewel/BP_BossDoor.BP_BossDoor_C|GetKeysActivated (Variables|Default|GetBossDoor)) (Variables|Default|GetKeyToValidatte))
    (Default|UpdateKeysActivated (Variables|Default|GetBossDoor))
    (Variables|Default|SetDidActivateKey true)))

(event EventBeginPlay)

(event Collision|EventActorBeginOverlap
  (params (OtherActor :type Actor%20Object%20Reference)))

(event EventTick
  (params (DeltaSeconds :type Float%20%28single-precision%29)))

(fn ConstructionScript
  (bind _cube (Variables|Default|GetCube))
  (switch Utilities|FlowControl|Switch|SwitchonEnum_JewelKeyType (Variables|Default|GetKeyToValidatte)
    (:NewEnumerator0
      (Rendering|Material|SetMaterial _cube 0 "/Game/LevelPrototyping/Materials/MI_Solid_Blue.MI_Solid_Blue"))
    (:NewEnumerator1
      (Rendering|Material|SetMaterial _cube 0 "/Game/Material/M_SampleColor_InstGreen.M_SampleColor_InstGreen"))
    (:NewEnumerator2
      (Rendering|Material|SetMaterial _cube 0 "/Game/Material/M_SampleColor_InstRed.M_SampleColor_InstRed"))
    (:NewEnumerator3
      (Rendering|Material|SetMaterial _cube 0 "/Game/Material/M_SampleColor_InstYellow.M_SampleColor_InstYellow"))))