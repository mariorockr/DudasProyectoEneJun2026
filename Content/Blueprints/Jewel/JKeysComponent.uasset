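; JKeysComponent is a component that tracks which colored keys its owner has collected.
; AddKeyToSet adds a key enum to KeysSetContainer if absent, then prints every held key to screen as debug output.
; Four query functions report whether the blue, green, yellow or red key is in the set, each converting it to an array for the lookup.
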(event EventBeginPlay)

(event EventTick
  (params (DeltaSeconds :type Float%20%28single-precision%29)))

(fn AddKeytoSet
  (params (NewKeyToAdd :type Enum_JewelKeyType%20Enum :default "NewEnumerator0"))
  (bind _keyssetcontainer (Variables|Default|GetKeysSetContainer))
  (bind _result (Utilities|Set|ToArray (Variables|Default|GetKeysSetContainer)))
  (if (not (Utilities|Array|ContainsItem _result NewKeyToAdd))
    (Utilities|Set|Add _keyssetcontainer NewKeyToAdd)
    (bind _result_2 (Utilities|Set|ToArray _keyssetcontainer))
    (for _array_element _result_2
      (Development|PrintString (Utilities|String|EnumtoString _array_element)))))

(fn HaveBlueKey
  (bind _result (Utilities|Set|ToArray (Variables|Default|GetKeysSetContainer)))
  (return (Utilities|Array|ContainsItem _result "NewEnumerator0")))

(fn HaveGreenKey
  (bind _result (Utilities|Set|ToArray (Variables|Default|GetKeysSetContainer)))
  (return (Utilities|Array|ContainsItem _result "NewEnumerator1")))

(fn HaveYellowKey
  (bind _result (Utilities|Set|ToArray (Variables|Default|GetKeysSetContainer)))
  (return (Utilities|Array|ContainsItem _result "NewEnumerator3")))

(fn HaveRedKey
  (bind _result (Utilities|Set|ToArray (Variables|Default|GetKeysSetContainer)))
  (return (Utilities|Array|ContainsItem _result "NewEnumerator2")))