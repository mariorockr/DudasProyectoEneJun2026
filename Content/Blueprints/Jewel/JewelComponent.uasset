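; Component that tracks which colored jewels its owner holds and which one is currently active.
; Adding a jewel not already in the enum set stores it, makes it active and prints the whole set as debug output.
; Getters expose per-color checks for blue, yellow, red and green, the jewel array, the active jewel and a HaveJewels value that no graph here updates.
; SwitchCurrentJewel is an unfinished stub.
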(event EventBeginPlay)

(event EventTick
  (params (DeltaSeconds :type Float%20%28single-precision%29)))

(fn AddJeweltoSet
  (params (NewJewel :type JewelType%20Enum :default "NewEnumerator0"))
  (bind _jewelsetcontainer (Variables|Default|GetJewelSetContainer))
  (bind _result (Utilities|Set|ToArray (Variables|Default|GetJewelSetContainer)))
  (if (not (Utilities|Array|ContainsItem _result NewJewel))
    (Variables|Default|SetCurrentActiveJewel NewJewel)
    (Utilities|Set|Add _jewelsetcontainer NewJewel)
    (bind _result_2 (Utilities|Set|ToArray _jewelsetcontainer))
    (for _array_element _result_2
      (Development|PrintString (Utilities|String|EnumtoString _array_element)))))

(fn HaveBlueJewel
  (bind _result (Utilities|Set|ToArray (Variables|Default|GetJewelSetContainer)))
  (return (Utilities|Array|ContainsItem _result "NewEnumerator0")))

(fn HaveYellowJewel
  (bind _result (Utilities|Set|ToArray (Variables|Default|GetJewelSetContainer)))
  (return (Utilities|Array|ContainsItem _result "NewEnumerator3")))

(fn HaveRedJewel
  (bind _result (Utilities|Set|ToArray (Variables|Default|GetJewelSetContainer)))
  (return (Utilities|Array|ContainsItem _result "NewEnumerator2")))

(fn HaveGreenJewel
  (bind _result (Utilities|Set|ToArray (Variables|Default|GetJewelSetContainer)))
  (return (Utilities|Array|ContainsItem _result "NewEnumerator1")))

(fn GetCurrentJewelsArray
  (bind _result (Utilities|Set|ToArray (Variables|Default|GetJewelSetContainer)))
  (return _result))

(fn GetHaveJewels
  (return (Variables|Default|GetHaveJewels)))

(fn SwitchCurrentJewel
  (Utilities|Set|ToArray (Variables|Default|GetJewelSetContainer)))

(fn GetCurrentActiveJewel
  (return (Variables|Default|GetCurrentActiveJewel)))