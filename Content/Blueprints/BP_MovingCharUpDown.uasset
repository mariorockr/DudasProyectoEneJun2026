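; Actor Blueprint that moves a Cube component vertically in an endless loop.
; On BeginPlay it caches the Cube's world transform, then a Timeline track drives a Z offset from that cached location, printing the value each update.
; When the Timeline finishes, the Cube snaps back to its cached transform and a custom ResetTimeline event replays it from the start.
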(event Custom|ResetTimeline
  (bind _cubetransform (Variables|Default|GetCubeTransform))
  (bind _newtrack_0 (Timeline|Timeline PlayFromStart)
    (:Update
      (Development|PrintString (Utilities|String|ToString(Float) _newtrack_0))
      (Transformation|SetWorldTransform (Variables|Default|GetCube) (Math|Transform|MakeTransform (Math|Vector|MakeVector (.x (.location _cubetransform)) (.y (.location _cubetransform)) (+ (.z (.location _cubetransform)) _newtrack_0)) "0, 0, 0" "1.000000,1.000000,1.000000") false false))
    (:Finished
      (Transformation|SetWorldTransform (Variables|Default|GetCube) (Variables|Default|GetCubeTransform) false false)
      (CallFunction|ResetTimeline))))

(event EventBeginPlay
  (Variables|Default|SetCubeTransform (Transformation|GetWorldTransform (Variables|Default|GetCube)))
  (bind _newtrack_0 (Timeline|Timeline PlayFromStart)
    (:Update
      (Development|PrintString (Utilities|String|ToString(Float) _newtrack_0))
      (Transformation|SetWorldTransform (Variables|Default|GetCube) (Math|Transform|MakeTransform (Math|Vector|MakeVector (.x (.location (Variables|Default|GetCubeTransform))) (.y (.location (Variables|Default|GetCubeTransform))) (+ (.z (.location (Variables|Default|GetCubeTransform))) _newtrack_0)) "0, 0, 0" "1.000000,1.000000,1.000000") false false))
    (:Finished
      (Transformation|SetWorldTransform (Variables|Default|GetCube) (Variables|Default|GetCubeTransform) false false)
      (CallFunction|ResetTimeline))))

(event Collision|EventActorBeginOverlap
  (params (OtherActor :type Actor%20Object%20Reference)))

(event EventTick
  (params (DeltaSeconds :type Float%20%28single-precision%29)))

(fn ConstructionScript)