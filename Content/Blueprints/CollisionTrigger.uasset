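; Box trigger that reveals a target actor while ColorItems covering all three required item types are inside it.
; BeginPlay builds the required-type set from a fixed list and hides ObjectToActivate.
; Overlap events track the items inside, re-run validation, print debug results and toggle the target's visibility.
; ValidateItems collects the present types into a temporary set, so duplicates and extra types do not affect the check.
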(event OnComponentBeginOverlap(Box)
  (params (OverlappedComponent :type Primitive%20Component%20Object%20Reference) (OtherActor :type Actor%20Object%20Reference) (OtherComp :type Primitive%20Component%20Object%20Reference) (OtherBodyIndex :type Integer) (bFromSweep :type Boolean) (SweepResult :type Hit%20Result%20Structure%20%28by%20ref%29))
  (bind _itemsinside (Variables|Default|GetItemsInside))
  (bind _ascolor_item (Utilities|Casting|CastToColorItem OtherActor))
  (Utilities|Array|AddUnique _itemsinside _ascolor_item)
  (for _array_element _itemsinside
    (Development|PrintString (Utilities|GetObjectName _array_element))
    (bind _isvalid (CallFunction|ValidateItems (Variables|Default|GetItemsInside)))
    (Development|PrintString (Utilities|String|ToString(Boolean) _isvalid))
    (Rendering|SetActorHiddenInGame (Variables|Default|GetObjectToActivate) (not _isvalid))))

(event OnComponentEndOverlap(Box)
  (params (OverlappedComponent :type Primitive%20Component%20Object%20Reference) (OtherActor :type Actor%20Object%20Reference) (OtherComp :type Primitive%20Component%20Object%20Reference) (OtherBodyIndex :type Integer))
  (bind _ascolor_item (Utilities|Casting|CastToColorItem OtherActor))
  (if (Utilities|Array|ContainsItem (Variables|Default|GetItemsInside) _ascolor_item)
    (Utilities|Array|RemoveItem (Variables|Default|GetItemsInside) _ascolor_item)
    (bind _isvalid (CallFunction|ValidateItems (Variables|Default|GetItemsInside)))
    (Development|PrintString (Utilities|String|ToString(Boolean) _isvalid))
    (Rendering|SetActorHiddenInGame (Variables|Default|GetObjectToActivate) (not _isvalid))))

(event EventBeginPlay
  (bind _output_get (Variables|Default|SetRequiredTypes (Utilities|Array|MakeArray "NewEnumerator0" "NewEnumerator1" "NewEnumerator2")))
  (for _array_element _output_get
    (Utilities|Set|Add (Variables|Default|GetRequiredTypesSet) _array_element)
    (bind _objecttoactivate (Variables|Default|GetObjectToActivate)
      (:then
        (Rendering|SetActorHiddenInGame _objecttoactivate true))
      (:else))))

(event Collision|EventActorBeginOverlap
  (params (OtherActor :type Actor%20Object%20Reference)))

(event EventTick
  (params (DeltaSeconds :type Float%20%28single-precision%29)))

(fn ConstructionScript)

(fn ValidateItems
  (params (ItemsToValidate :type Array%20of%20Color%20Item%20Object%20References))
  (Utilities|Set|Clear (Variables|Default|GetTemporalTypesSet))
  (for _array_element ItemsToValidate
    (if (not (Utilities|Set|Contains (Variables|Default|GetTemporalTypesSet) (Variables|/Game/Blueprints/ColorItem.ColorItem_C|GetItemType _array_element)))
      (Utilities|Set|Add (Variables|Default|GetTemporalTypesSet) (Variables|/Game/Blueprints/ColorItem.ColorItem_C|GetItemType _array_element))))
  (bind _result (Utilities|Set|ToArray (Variables|Default|GetRequiredTypesSet)))
  (for _array_element_2 _result
    (if (not (Utilities|Set|Contains (Variables|Default|GetTemporalTypesSet) _array_element_2))
      (return false)))
  (return true))